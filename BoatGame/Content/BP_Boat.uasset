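; BP_Boat is the boat actor that owns the game's HUD and switches the scene between day and evening.
; It creates BP_HUD on BeginPlay, and its events forward game start, points, crash, turn sign and reset to that widget.
; ToggleAtmosphere flips IsEvening, then sets fog color through a material parameter collection, adjusts directional and sky light intensity, and passes the state to BP_ProceduralPlatformGenerator.
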(event EventBeginPlay
  (bind _returnvalue (UserInterface|CreateWidget "/Game/BP_HUD.BP_HUD_C" 0 self))
  (bind _output_get (Variables|Default|SetHUD _returnvalue))
  (UserInterface|Viewport|AddtoViewport _output_get 0))

(event EventUpdatePointText
  (params (PointCount :type Integer))
  (Default|SetPointText (Variables|Default|GetHUD) PointCount))

(event EventStartHUD
  (Default|StartGame (Variables|Default|GetHUD)))

(event EventUpdateHUDonCrash
  (Default|PlayCrashAnim (Variables|Default|GetHUD)))

(event EventShowTurnSigninHUD
  (Default|ShowTurnSign (Variables|Default|GetHUD)))

(event EventResetHUD
  (Default|ResetUI (Variables|Default|GetHUD)))

(fn ConstructionScript)

(fn ToggleAtmosphere
  (bind _output_get (Variables|Default|SetIsEvening (not (Variables|Default|GetIsEvening))))
  (if _output_get
    (Rendering|Material|SetVectorParameterValue "/Game/Assets/Environment/Materials/PPVPC.PPVPC" "FogColor" (Utilities|Struct|MakeLinearColor 0.65 0.58 0.58 1.0) :!class /Script/Engine.KismetMaterialLibrary)
    (bind _returnvalue (Actor|GetActorOfClass "/Script/Engine.DirectionalLight"))
    (Rendering|Components|Light|SetIntensity (Variables|/Script/Engine.Light|GetLightComponent _returnvalue) 0.5)
    (bind _returnvalue_2 (Actor|GetActorOfClass "/Script/Engine.SkyLight"))
    (Rendering|Components|Light|SetIntensity (Variables|/Script/Engine.SkyLight|GetLightComponent _returnvalue_2) 0.6)
    (bind _returnvalue_3 (Actor|GetActorOfClass "/Game/BP_ProceduralPlatformGenerator.BP_ProceduralPlatformGenerator_C"))
    (Default|SetIsIsEvening _returnvalue_3 1.0)
    (else
      (Rendering|Material|SetVectorParameterValue "/Game/Assets/Environment/Materials/PPVPC.PPVPC" "FogColor" (Utilities|Struct|MakeLinearColor 0.85 0.75 0.75 1.0) :!class /Script/Engine.KismetMaterialLibrary)
      (bind _returnvalue_4 (Actor|GetActorOfClass "/Script/Engine.DirectionalLight"))
      (Rendering|Components|Light|SetIntensity (Variables|/Script/Engine.Light|GetLightComponent _returnvalue_4) 3.0)
      (bind _returnvalue_5 (Actor|GetActorOfClass "/Script/Engine.SkyLight"))
      (Rendering|Components|Light|SetIntensity (Variables|/Script/Engine.SkyLight|GetLightComponent _returnvalue_5) 1.0)
      (bind _returnvalue_6 (Actor|GetActorOfClass "/Game/BP_ProceduralPlatformGenerator.BP_ProceduralPlatformGenerator_C"))
      (Default|SetIsIsEvening _returnvalue_6 0.0))))