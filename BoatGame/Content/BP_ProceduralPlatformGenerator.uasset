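; BP_ProceduralPlatformGenerator prepares the instanced-mesh components for procedural platform obstacles, people and environment items.
; Its construction script creates one static, shadowless HISM component per mesh in each asset array, with collision only on obstacles, then calls SetupCustomData.
; Environment items share a dynamic M_PolygonCity material, whose IsEvening parameter SetIsIsEvening sets to switch the evening look.
; Instance placement is not part of these graphs.
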(fn ConstructionScript
  (bind _environmentitems (Variables|Default|GetEnvironmentItems))
  (bind _environmentitems_2 (Variables|Default|GetEnvironmentItems))
  (bind _obstacles (Variables|Default|GetObstacles))
  (bind _obstacles_2 (Variables|Default|GetObstacles))
  (bind _people (Variables|Default|GetPeople))
  (bind _people_2 (Variables|Default|GetPeople))
  (bind _returnvalue (Rendering|Material|CreateDynamicMaterialInstance "/Game/Assets/Environment/Materials/M_PolygonCity.M_PolygonCity" "None" "None" :!class /Script/Engine.KismetMaterialLibrary))
  (Variables|Default|SetM_PolygonCity _returnvalue)
  (Utilities|FlowControl|Sequence
    (:then_0
      (Utilities|Array|Resize _obstacles (Utilities|Array|Length (LocalVariables|GetObstacleAssets)))
      (for _index (range 0 (Utilities|Array|LastIndex _obstacles))
        (bind _returnvalue_2 (AddComponent|AddHierarchicalInstancedStaticMeshComponent false))
        (Utilities|Array|SetArrayElem _obstacles_2 _index _returnvalue_2)
        (Transformation|SetMobility (Utilities|Array|Get(acopy) _obstacles_2 _index) "Static")
        (Components|StaticMesh|SetStaticMesh (Utilities|Array|Get(acopy) _obstacles_2 _index) (Utilities|Array|Get(acopy) (LocalVariables|GetObstacleAssets) _index))
        (Components|Tick|SetComponentTickEnabled (Utilities|Array|Get(acopy) _obstacles_2 _index) false)
        (Variables|/Script/Engine.PrimitiveComponent|SetbGenerateOverlapEvents (Utilities|Array|Get(acopy) _obstacles_2 _index) false)
        (Variables|/Script/Engine.PrimitiveComponent|SetCanCharacterStepUpOn (Utilities|Array|Get(acopy) _obstacles_2 _index) "ECB_No")
        (Collision|SetCollisionProfileName (Utilities|Array|Get(acopy) _obstacles_2 _index) "Obstacle" false :!class /Script/Engine.PrimitiveComponent)
        (Rendering|SetCastShadow (Utilities|Array|Get(acopy) _obstacles_2 _index) false)))
    (:then_1
      (Utilities|Array|Resize _people (Utilities|Array|Length (LocalVariables|GetPeopleAssets)))
      (for _index_2 (range 0 (Utilities|Array|LastIndex _people))
        (bind _returnvalue_3 (AddComponent|AddHierarchicalInstancedStaticMeshComponent false))
        (Utilities|Array|SetArrayElem _people_2 _index_2 _returnvalue_3)
        (Transformation|SetMobility (Utilities|Array|Get(acopy) _people_2 _index_2) "Static")
        (Components|StaticMesh|SetStaticMesh (Utilities|Array|Get(acopy) _people_2 _index_2) (Utilities|Array|Get(acopy) (LocalVariables|GetPeopleAssets) _index_2))
        (Components|Tick|SetComponentTickEnabled (Utilities|Array|Get(acopy) _people_2 _index_2) false)
        (Variables|/Script/Engine.PrimitiveComponent|SetbGenerateOverlapEvents (Utilities|Array|Get(acopy) _people_2 _index_2) false)
        (Variables|/Script/Engine.PrimitiveComponent|SetCanCharacterStepUpOn (Utilities|Array|Get(acopy) _people_2 _index_2) "ECB_No")
        (Collision|SetCollisionProfileName (Utilities|Array|Get(acopy) _people_2 _index_2) "NoCollision" false :!class /Script/Engine.PrimitiveComponent)
        (Rendering|SetCastShadow (Utilities|Array|Get(acopy) _people_2 _index_2) false)))
    (:then_2
      (Utilities|Array|Resize _environmentitems_2 (Utilities|Array|Length (LocalVariables|GetEnvironmentAssets)))
      (for _index_3 (range 0 (Utilities|Array|LastIndex _environmentitems_2))
        (bind _returnvalue_4 (AddComponent|AddHierarchicalInstancedStaticMeshComponent false))
        (Utilities|Array|SetArrayElem _environmentitems _index_3 _returnvalue_4)
        (Transformation|SetMobility (Utilities|Array|Get(acopy) _environmentitems _index_3) "Static")
        (Components|StaticMesh|SetStaticMesh (Utilities|Array|Get(acopy) _environmentitems _index_3) (Utilities|Array|Get(acopy) (LocalVariables|GetEnvironmentAssets) _index_3))
        (Rendering|Material|SetMaterial (Utilities|Array|Get(acopy) _environmentitems _index_3) 0 (Variables|Default|GetM_PolygonCity))
        (Components|Tick|SetComponentTickEnabled (Utilities|Array|Get(acopy) _environmentitems _index_3) false)
        (Variables|/Script/Engine.PrimitiveComponent|SetbGenerateOverlapEvents (Utilities|Array|Get(acopy) _environmentitems _index_3) false)
        (Collision|SetCollisionProfileName (Utilities|Array|Get(acopy) _environmentitems _index_3) "NoCollision" false :!class /Script/Engine.PrimitiveComponent)
        (Rendering|SetCastShadow (Utilities|Array|Get(acopy) _environmentitems _index_3) false)))
    (:then_3
      (Class|ProceduralPlatformGeneratorBase|SetupCustomData))))

(fn SetIsIsEvening
  (params (Value :type Float%20%28single-precision%29))
  (Rendering|Material|SetScalarParameterValue (Variables|Default|GetM_PolygonCity) "IsEvening" Value :!class /Script/Engine.MaterialInstanceDynamic))